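; BP_Seeker is a seeker character that supplies looping patrol points based on where it starts.
; On BeginPlay it caches its location and rotation as the patrol origin.
; GetPatrolPoint adds the indexed PatrolPoints offset to that origin, rotates the whole sum by the starting rotation, and returns it with the next index, wrapping to zero.
; No movement logic lives in this Blueprint.
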(event EventBeginPlay
  (Variables|Patrol|SetPatrolOrigin (Transformation|GetActorLocation))
  (Variables|Patrol|SetPatrolOriginRotation (Transformation|GetActorRotation)))

(event Collision|EventActorBeginOverlap
  (params (OtherActor :type Actor%20Object%20Reference)))

(event EventTick
  (params (DeltaSeconds :type Float%20%28single-precision%29)))

(fn ConstructionScript)

(fn GetPatrolPoint
  (params (CurrentIndex :type Integer))
  (bind _patrolpoints (Variables|Patrol|GetPatrolPoints))
  (LocalVariables|SetNextPatrolPoint (Math|Vector|RotateVector (+ (Variables|Patrol|GetPatrolOrigin) (Utilities|Array|Get(acopy) _patrolpoints CurrentIndex)) (Variables|Patrol|GetPatrolOriginRotation)))
  (bind _result (Math|Integer|IncrementInt CurrentIndex)
    (:%20%20
      (if (>= _result (Utilities|Array|Length _patrolpoints))
        (return (LocalVariables|GetNextPatrolPoint) 0)
        (else
          (return (LocalVariables|GetNextPatrolPoint) CurrentIndex))))))